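; Player controller Blueprint containing currently disabled Tick logic for turning the controlled pawn to face the mouse cursor.
; That logic deprojects the mouse onto a horizontal plane at the pawn's height and applies a look-at rotation.
; The MoveCursor graph holds ray-plane intersection math, shown unconnected, and a BP_TestCharacter Died check is disabled and unreachable.
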(event EventTick
  (params (DeltaSeconds :type Float%20%28single-precision%29))
  (bind (_worldlocation _worlddirection) (Game|Player|ConvertMouseLocationToWorldSpace))
  (bind _returnvalue (Pawn|GetControlledPawn))
  (bind _returnvalue_2 (Transformation|GetActorLocation _returnvalue))
  (if true
    (Transformation|SetActorRotation (Pawn|GetControlledPawn) (Math|Rotator|FindLookatRotation _returnvalue_2 (.Intersection%20Point (Utilities|MoveCursor _worldlocation _worlddirection 5e+04 _returnvalue_2 "0,0,1.000000"))))))

(fn ConstructionScript)